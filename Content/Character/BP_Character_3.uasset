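; BP_Character_3 is a character that automatically shuttles back and forth using navigation moves.
; A looping timer started on BeginPlay periodically sends its instigator controller to LocationTo via SimpleMoveToLocation.
; After a short delay within each cycle, a second move redirects it to a point behind its current position, computed from the reversed forward vector.
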(event `self.ReceiveBeginPlay`
  (`KismetSystemLibrary.K2_SetTimerDelegate` (delegate `MoveBackOnTimer`) 1.5 true))

(event `MoveBackOnTimer`
  (`AIBlueprintHelperLibrary.SimpleMoveToLocation` (`self.GetInstigatorController`) (`self.LocationTo`))
  (`KismetSystemLibrary.Delay` 1.0)
  (`AIBlueprintHelperLibrary.SimpleMoveToLocation` (`self.GetInstigatorController`) (+ (* (`self.GetActorForwardVector`) -1000.0) (`self.K2_GetActorLocation`))))

(fn `UserConstructionScript`)